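; Key pickup actor that the first-person player carries and uses to remove doors.
; Overlapping its sphere snaps it to the character's GripPoint socket and binds to that character's OnUseItem dispatcher.
; UseKey line-traces from the key along the player camera's forward vector and destroys the hit actor if it is tagged "Door", avoiding a hard reference to a door class.
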(event OnComponentBeginOverlap(SphereCollision)
  (params (OverlappedComponent :type Primitive%20Component%20Object%20Reference) (OtherActor :type Actor%20Object%20Reference) (OtherComp :type Primitive%20Component%20Object%20Reference) (OtherBodyIndex :type Integer) (bFromSweep :type Boolean) (SweepResult :type Hit%20Result%20Structure%20%28by%20ref%29))
  (bind _asbp_first_person_character (Utilities|Casting|CastToBP_FirstPersonCharacter OtherActor))
  (Transformation|AttachComponentToComponent self (Variables|/Game/StarterStuff/FirstPerson/Blueprints/BP_FirstPersonCharacter.BP_FirstPersonCharacter_C|GetFirstPersonMesh _asbp_first_person_character) "GripPoint" "SnapToTarget" "SnapToTarget" "KeepWorld" true)
  (EventDispatchers|AssignOnUseItem _asbp_first_person_character (EventDispatchers|CreateEvent :!event Custom|UseKey)))

(event Custom|UseKey
  (bind _returnvalue (Transformation|GetActorLocation))
  (bind _outhit (Collision|LineTraceByChannel _returnvalue (+ _returnvalue (* (Math|Vector|GetForwardVector (Camera|GetCameraRotation (Game|GetPlayerCameraManager 0))) "1000.000000,1000.000000,1000.000000")) "TraceTypeQuery1" false 0 "None"))
  (Utilities|IsValid (.hitactor _outhit)
    (:Is%20Valid
      (if (Actor|ActorHasTag (.hitactor _outhit) "Door")
        (Actor|DestroyActor (.hitactor _outhit))))))

(event EventBeginPlay)

(event EventTick
  (params (DeltaSeconds :type Float%20%28single-precision%29)))

(fn ConstructionScript)